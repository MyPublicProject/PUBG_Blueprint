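; World map component that creates the map UI, toggles it with cursor and input mode, and shows the player and clickable markers.
; Two corner actors define the world bounds used to convert between world locations and map pixels.
; The player icon updates on movement and on a timer while jumping; zooming rescales the map and optionally the icons.
; Clicks trace down to spawn marker actors with cycling colors, replacing the oldest at the limit.
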(event Custom|InitializeMap
  (params (Player :type Character%20Object%20Reference))
  (Utilities|IsValid Player
    (:Is%20Valid
      (Variables|Default|SetPlayer Player)
      (bind _returnvalue (UserInterface|CreateWidget "/Game/Interface/MapUI/W_Man.W_Man_C"))
      (bind _output_get (Variables|Default|SetMainReference _returnvalue))
      (bind _output_get_2 (Variables|Default|SetMapReference (Variables|/Game/Interface/MapUI/W_Man.W_Man_C|GetWorldMap _output_get)))
      (Default|Initialize _output_get_2 self)
      (Variables|Default|SetOriginalPlayerSize (Math|Vector2D|MakeVector2D (Math|Conversions|ToFloat(Integer) (Variables|/Game/Interface/MapUI/W_WorldMap.W_WorldMap_C|GetPlayerSizeX (Variables|Default|GetMapReference))) (Math|Conversions|ToFloat(Integer) (Variables|/Game/Interface/MapUI/W_WorldMap.W_WorldMap_C|GetPlayerSizeY (Variables|Default|GetMapReference)))))
      (Variables|Default|SetOriginalMapSize (Math|Vector2D|MakeVector2D (Math|Conversions|ToFloat(Integer) (Variables|/Game/Interface/MapUI/W_WorldMap.W_WorldMap_C|GetMapSizeX (Variables|Default|GetMapReference))) (Math|Conversions|ToFloat(Integer) (Variables|/Game/Interface/MapUI/W_WorldMap.W_WorldMap_C|GetMapSizeY (Variables|Default|GetMapReference)))))
      (Variables|Settings|SetOriginalMarkerSize (Variables|Settings|GetMarkerSize))
      (Variables|Default|SetAvailableColors (Variables|Settings|GetMarkerColors))
      (CallFunction|ShowMap false)
      (UserInterface|Viewport|AddtoViewport (Variables|Default|GetMainReference) 0))
    (:Is%20Not%20Valid
      (Development|PrintString "该加班了！！程序猿" true true "(R=1.000000,G=0.000000,B=0.000000,A=1.000000)" 1e+02))))

(event Custom|OnPlayerMoved
  (if (Variables|Default|GetVisible?)
    (CallFunction|UpdatePlayerPositiononMap)))

(event Custom|OnPlayerJump
  (Variables|Default|SetJumpimg? true)
  (if (Variables|Default|GetVisible?)
    (bind _returnvalue (Utilities|Time|SetTimerbyFunctionName self "UpdatePlayerPositionOnMap" (Variables|Settings|GetInAirUpdateRate) true)) ; 设置时间内循环调用某个函数
    (Variables|Default|SetUpdateTimerHandle _returnvalue)))

(event Custom|StartTimer
  (bind _returnvalue (Utilities|Time|SetTimerbyFunctionName self "UpdatePlayerPositionOnMap" (Variables|Settings|GetInAirUpdateRate) true)) ; 设置时间内循环调用某个函数
  (Variables|Default|SetUpdateTimerHandle _returnvalue))

(event Custom|OnPlayerLand
  (Variables|Default|SetJumpimg? false)
  (if (Utilities|Time|IsValidTimerHandle (Variables|Default|GetUpdateTimerHandle))
    (Utilities|Time|ClearandInvalidateTimerbyHandle (Variables|Default|GetUpdateTimerHandle))
    (CallFunction|UpdatePlayerPositiononMap)))

(event Custom|Oninputmodifysize
  (params (Increase? :type Boolean) (Percent :type Integer))
  (bind _mapreference (Variables|Default|GetMapReference))
  (if (Variables|Default|GetVisible?)
    (CallFunction|ModifyMapSize (+ 1.0 (* (Math|Conversions|ToFloat(Integer) (Math|Integer|SelectInt 1 -1 Increase?)) (/ (Math|Conversions|ToFloat(Integer) (Math|Integer|Clamp(Integer) Percent 0 100)) 1e+02))))
    (if Increase?
      (Class|Widget|SetRenderTranslation (Variables|/Game/Interface/MapUI/W_WorldMap.W_WorldMap_C|GetMapOverlay _mapreference) (* (Utilities|Struct|BreakWidgetTransform (Variables|/Script/UMG.Widget|GetRenderTransform _mapreference)) (Variables|Default|GetCurrentSizeMultiplier))))))

(event Custom|OnMapClicked
  (params (Position :type Vector%202D%20Structure))
  (bind _location (CallFunction|MapPositiontoWorldLocation Position))
  (bind _out (CallFunction|TraceDownWorldLocation _location))
  (Math|Integer|CompareInt (Variables|Settings|GetMaxAmountOfMakers)
    (:>
      (if (>= (Utilities|Array|Length (Variables|Default|GetCurrentMarkers)) (Variables|Settings|GetMaxAmountOfMakers))
        (CallFunction|RemoveMarkerbyIndex)))
    (:<
      _))
  (bind _returnvalue (Game|SpawnActorfromClass "/Game/Interface/MapUI/Database/BP_Marker.BP_Marker_C" (Math|Transform|MakeTransform _out "0, 0, 0" "1,1,1") "Undefined" 0 0))
  (bind _out_2 (CallFunction|PickMarkerColor))
  (CallFunction|AddMarker (Utilities|Struct|MakeS_MarkerInfo _out 0 _out_2 _returnvalue)))

(fn GetMapHeight
  (bind _lowerrightcorner (Variables|Settings|GetLowerRightCorner))
  (bind _upperleftcorner (Variables|Settings|GetUpperLeftCorner))
  (Utilities|IsValid _lowerrightcorner
    (:Is%20Valid
      (Utilities|IsValid _upperleftcorner
        (:Is%20Valid
          (return (Math|Float|Absolute(Float) (- (.X (Math|Vector|BreakVector (Transformation|GetActorLocation _lowerrightcorner))) (.X (Math|Vector|BreakVector (Transformation|GetActorLocation _upperleftcorner)))))))))))

(fn GetMapWidth
  (bind _lowerrightcorner (Variables|Settings|GetLowerRightCorner))
  (bind _upperleftcorner (Variables|Settings|GetUpperLeftCorner))
  (Utilities|IsValid _lowerrightcorner
    (:Is%20Valid
      (Utilities|IsValid _upperleftcorner
        (:Is%20Valid
          (return (Math|Float|Absolute(Float) (- (.Y (Math|Vector|BreakVector (Transformation|GetActorLocation _lowerrightcorner))) (.Y (Math|Vector|BreakVector (Transformation|GetActorLocation _upperleftcorner)))))))))))

(fn ConvertLocationtoMapLocation
  (params (Location :type Vector))
  (bind (_x _y) (Math|Vector|BreakVector Location))
  (bind _upperleftcorner (Variables|Settings|GetUpperLeftCorner))
  (bind _returnvalue (Transformation|GetActorLocation _upperleftcorner))
  (bind (_x_2 _y_2) (Math|Vector|BreakVector _returnvalue))
  (Utilities|IsValid _upperleftcorner
    (:Is%20Valid
      (return (Math|Vector2D|MakeVector2D (Math|Float|Absolute(Float) (- _y _y_2)) (Math|Float|Absolute(Float) (- _x _x_2)))))))

(fn ShowMap
  (params (Show? :type Boolean))
  (bind _returnvalue (Game|GetPlayerController 0))
  (bind _returnvalue_2 (Game|GetPlayerController 0))
  (if (Math|Boolean|NotEqual(Boolean) Show? (Variables|Default|GetVisible?))
    (bind _output_get (Variables|Default|SetVisible? Show?))
    (if _output_get
      (Widget|SetVisibility (Variables|Default|GetMapReference) "SelfHitTestInvisible")
      (Variables|/Script/Engine.PlayerController|SetbShowMouseCursor _returnvalue_2 true)
      (Input|SetInputModeGameandUI _returnvalue_2 (Variables|Default|GetMainReference) "DoNotLock" false)
      (CallFunction|UpdatePlayerPositiononMap)
      (return)
      (else
        (Widget|SetVisibility (Variables|Default|GetMapReference) "Hidden")
        (Variables|/Script/Engine.PlayerController|SetbShowMouseCursor _returnvalue false)
        (Input|SetInputModeGameOnly _returnvalue)
        (return)))
    (else
      (return))))

(fn ToggleVisibility
  (CallFunction|ShowMap (not (Variables|Default|GetVisible?)))
  (if (and (Variables|Default|GetVisible?) (Variables|Default|GetJumpimg?))
    (CallFunction|StartTimer)
    (return)
    (elif (and (not (Variables|Default|GetVisible?)) (Utilities|Time|IsValidTimerHandle (Variables|Default|GetUpdateTimerHandle)))
      (Utilities|Time|ClearandInvalidateTimerbyHandle (Variables|Default|GetUpdateTimerHandle))
      (return)
      (else
        (return)))))

(fn LocationtoMapPosition
  (params (Location :type Vector) (WidgetSize :type Vector%202D%20Structure))
  (bind _out (CallFunction|ConvertLocationtoMapLocation Location))
  (bind (_x _y) (Math|Vector2D|BreakVector2D WidgetSize))
  (bind _mapreference (Variables|Default|GetMapReference))
  (bind _mapreference_2 (Variables|Default|GetMapReference))
  (bind (_x_2 _y_2) (Math|Vector2D|BreakVector2D _out))
  (Utilities|IsValid _mapreference
    (:Is%20Valid
      (Utilities|IsValid _mapreference_2
        (:Is%20Valid
          (return (Math|Vector2D|MakeVector2D (- (* (/ _x_2 (CallFunction|GetMapWidth)) (Math|Conversions|ToFloat(Integer) (Variables|/Game/Interface/MapUI/W_WorldMap.W_WorldMap_C|GetMapSizeX _mapreference))) (/ _x 2.0)) (- (* (/ _y_2 (CallFunction|GetMapHeight)) (Math|Conversions|ToFloat(Integer) (Variables|/Game/Interface/MapUI/W_WorldMap.W_WorldMap_C|GetMapSizeY _mapreference_2))) (/ _y 2.0)))))))))

(fn UpdatePlayerPositiononMap
  (bind _player (Variables|Default|GetPlayer))
  (bind _originalplayersize (Variables|Default|GetOriginalPlayerSize))
  (Utilities|IsValid _player
    (:Is%20Valid
      (Class|Widget|SetRenderTranslation (Variables|/Game/Interface/MapUI/W_WorldMap.W_WorldMap_C|GetPlayerBox (Variables|Default|GetMapReference)) (CallFunction|LocationtoMapPosition (Transformation|GetActorLocation _player) (select (Variables|Settings|GetKeepPlayerSizeWhenZooming?) _originalplayersize (* _originalplayersize (Variables|Default|GetCurrentSizeMultiplier)))))
      (return))))

(fn ModifyMapSize
  (params (Multiplier :type Float%20%28single-precision%29))
  (if (>= Multiplier 0.0)
    (Variables|Default|SetCurrentSizeMultiplier (Math|Float|Clamp(Float) (* Multiplier (Variables|Default|GetCurrentSizeMultiplier)) (Variables|Settings|GetMinZoom) (Variables|Settings|GetMaxZoom)))
    (Default|SetMapSize (Variables|Default|GetMapReference) (Math|Float|Round (.X (Math|Vector2D|BreakVector2D (* (Variables|Default|GetOriginalMapSize) (Variables|Default|GetCurrentSizeMultiplier))))) (Math|Float|Round (.Y (Math|Vector2D|BreakVector2D (* (Variables|Default|GetOriginalMapSize) (Variables|Default|GetCurrentSizeMultiplier))))))
    (if (Variables|Settings|GetKeepPlayerSizeWhenZooming?)
      _
      (else
        (Default|SetPlayerSize (Variables|Default|GetMapReference) (Math|Float|Round (.X (Math|Vector2D|BreakVector2D (* (Variables|Default|GetOriginalPlayerSize) (Variables|Default|GetCurrentSizeMultiplier))))) (Math|Float|Round (.Y (Math|Vector2D|BreakVector2D (* (Variables|Default|GetOriginalPlayerSize) (Variables|Default|GetCurrentSizeMultiplier))))))))
    (CallFunction|UpdatePlayerPositiononMap)
    (if (Variables|Settings|GetKeepMarkerSizeWhenZooming?)
      _
      (else
        (Variables|Settings|SetMarkerSize (Math|Float|Round (* (Variables|Settings|GetOriginalMarkerSize) (Variables|Default|GetCurrentSizeMultiplier))))
        (CallFunction|UpdateMarkerSizes)))
    (CallFunction|UpdateMarkerPositions)
    (return)
    (else
      (return))))

(fn MapOutOfBoundaries?
  (bind _returnvalue (Viewport|GetViewportSize))
  (bind _mapreference (Variables|Default|GetMapReference))
  (bind _returnvalue_2 (Class|Widget|GetDesiredSize _mapreference))
  (bind (_x _y) (Math|Vector2D|BreakVector2D _returnvalue))
  (bind (_x_2 _y_2) (Math|Vector2D|BreakVector2D _returnvalue_2))
  (return (or (> _x_2 _x) (> _y_2 _y))))

(fn AddMarker
  (params (Marker :type S%20Marker%20Info%20Structure))
  (bind (_worldlocation _widget _color) (Utilities|Struct|BreakS_MarkerInfo Marker))
  (bind _markersize (Variables|Settings|GetMarkerSize))
  (bind _returnvalue (Utilities|Array|Add (Variables|Default|GetCurrentMarkers) Marker))
  (LocalVariables|SetLocalIndex _returnvalue)
  (bind _widget_2 (Default|AddMarkertoMap (Variables|Default|GetMapReference) (LocalVariables|GetLocalIndex) _color self (CallFunction|LocationtoMapPosition _worldlocation (Math|Vector2D|MakeVector2D (Math|Conversions|ToFloat(Integer) _markersize) (Math|Conversions|ToFloat(Integer) _markersize)))))
  (Utilities|Struct|SetmembersinS_MarkerInfo (Utilities|Array|Get(acopy) (Variables|Default|GetCurrentMarkers) (LocalVariables|GetLocalIndex)) _widget_2)
  (return))

(fn MapPositiontoWorldLocation
  (params (Position :type Vector%202D%20Structure))
  (bind (_x _y) (Math|Vector2D|BreakVector2D Position))
  (bind _upperleftcorner (Variables|Settings|GetUpperLeftCorner))
  (bind _mapreference (Variables|Default|GetMapReference))
  (bind _returnvalue (Transformation|GetActorLocation _upperleftcorner))
  (bind (_x_2 _y_2) (Math|Vector|BreakVector _returnvalue))
  (LocalVariables|SetLocalPercentageInX (/ _x (Math|Conversions|ToFloat(Integer) (Variables|/Game/Interface/MapUI/W_WorldMap.W_WorldMap_C|GetMapSizeX _mapreference))))
  (LocalVariables|SetLocalPercentageInY (/ _y (Math|Conversions|ToFloat(Integer) (Variables|/Game/Interface/MapUI/W_WorldMap.W_WorldMap_C|GetMapSizeY _mapreference))))
  (return (Math|Vector|MakeVector (- _x_2 (* (CallFunction|GetMapHeight) (LocalVariables|GetLocalPercentageInY))) (+ _y_2 (* (Math|Float|Absolute(Float) (- (.Y (Math|Vector|BreakVector (Transformation|GetActorLocation (Variables|Settings|GetLowerRightCorner)))) (.Y (Math|Vector|BreakVector (Transformation|GetActorLocation (Variables|Settings|GetUpperLeftCorner)))))) (LocalVariables|GetLocalPercentageInX))) 0.0)))

(fn TraceDownWorldLocation
  (params (In :type Vector))
  (LocalVariables|SetLocation In)
  (bind (_outhit _returnvalue) (Collision|LineTraceByChannel (Math|Vector|MakeVector (.X (Math|Vector|BreakVector (LocalVariables|GetLocation))) (.Y (Math|Vector|BreakVector (LocalVariables|GetLocation))) (Variables|Settings|GetTranceDownHeight)) (LocalVariables|GetLocation) "TraceTypeQuery1" false 0 "None"))
  (if _returnvalue
    (return (.Location (Collision|BreakHitResult _outhit)))
    (else
      (return (LocalVariables|GetLocation)))))

(fn UpdateMarkerPositions
  (bind _markersize (Variables|Settings|GetMarkerSize))
  (for _array_element (Variables|Default|GetCurrentMarkers)
    (Utilities|IsValid (.Widget (Utilities|Struct|BreakS_MarkerInfo _array_element))
      (:Is%20Valid
        (Class|Widget|SetRenderTranslation (.Widget (Utilities|Struct|BreakS_MarkerInfo _array_element)) (CallFunction|LocationtoMapPosition (.WorldLocation (Utilities|Struct|BreakS_MarkerInfo _array_element)) (Math|Vector2D|MakeVector2D (Math|Conversions|ToFloat(Integer) _markersize) (Math|Conversions|ToFloat(Integer) _markersize)))))))
  (return))

(fn UpdateMarkerSizes
  (for _array_element (Variables|Default|GetCurrentMarkers)
    (Utilities|IsValid (Utilities|Struct|BreakS_MarkerInfo _array_element)
      (:Is%20Valid
        (Default|UpdateSize (Utilities|Struct|BreakS_MarkerInfo _array_element) (Variables|Settings|GetMarkerSize)))))
  (return))

(fn PickMarkerColor
  (LocalVariables|SetLocalCoolor (Utilities|Array|Get(acopy) (Variables|Default|GetAvailableColors)))
  (Utilities|Array|RemoveIndex (Variables|Default|GetAvailableColors))
  (if (<= (Utilities|Array|Length (Variables|Default|GetAvailableColors)) 0)
    (Variables|Default|SetAvailableColors (Variables|Settings|GetMarkerColors)))
  (return (LocalVariables|GetLocalCoolor)))

(fn RemoveMarkerbyIndex
  (params (Index :type Integer))
  (bind _currentmarkers (Variables|Default|GetCurrentMarkers))
  (bind _output (Utilities|Array|Get(acopy) _currentmarkers Index))
  (bind (_widget _color _markeractor) (Utilities|Struct|BreakS_MarkerInfo _output))
  (if (Utilities|Array|IsValidIndex (Variables|Default|GetCurrentMarkers) Index)
    (if (Utilities|Array|ContainsItem (Variables|Default|GetAvailableColors) _color)
      _
      (else
        (Utilities|Array|Insert (Variables|Default|GetAvailableColors) _color)))
    (Actor|DestroyActor _markeractor)
    (Widget|RemovefromParent _widget)
    (Utilities|Array|RemoveIndex (Variables|Default|GetCurrentMarkers) Index)
    (for (_array_element _array_index) (Variables|Default|GetCurrentMarkers)
      (Utilities|IsValid (Utilities|Struct|BreakS_MarkerInfo _array_element)
        (:Is%20Valid
          (Variables|/Game/Interface/MapUI/W_MARKER.W_Marker_C|SetIndex (Utilities|Struct|BreakS_MarkerInfo _array_element) _array_index))))
    (return)
    (else
      (return))))