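; BP_骨灰盒 (cremation urn) is an equipment item actor that notifies the player character when it comes within range.
; BeginPlay caches player 0's BP_Character as CharacterRef.
; When a BP_Character begins or ends overlap with the Box trigger, it passes GItemInfo to the cached character through GMeetMessage or GLeaveMessage, not to the overlapping actor itself.
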(event OnComponentBeginOverlap(Box)
  (params (OverlappedComponent :type Primitive%20Component%20Object%20Reference) (OtherActor :type Actor%20Object%20Reference) (OtherComp :type Primitive%20Component%20Object%20Reference) (OtherBodyIndex :type Integer) (bFromSweep :type Boolean) (SweepResult :type Hit%20Result%20Structure%20%28by%20ref%29))
  (bind _characterref (Variables|Default|GetCharacterRef))
  (Utilities|Casting|CastToBP_Character OtherActor)
  (Utilities|IsValid _characterref
    (:Is%20Valid
      (Class|BP骨灰数据|GMeet(Message) _characterref (Variables|Default|GetG_ItemInfo)))))

(event OnComponentEndOverlap(Box)
  (params (OverlappedComponent :type Primitive%20Component%20Object%20Reference) (OtherActor :type Actor%20Object%20Reference) (OtherComp :type Primitive%20Component%20Object%20Reference) (OtherBodyIndex :type Integer))
  (bind _characterref (Variables|Default|GetCharacterRef))
  (Utilities|Casting|CastToBP_Character OtherActor)
  (Utilities|IsValid _characterref
    (:Is%20Valid
      (Class|BP骨灰数据|GLeave(Message) _characterref (Variables|Default|GetG_ItemInfo)))))

(event EventBeginPlay
  ;[1 1 1] 初始化
  (bind _asbp_character (Utilities|Casting|CastToBP_Character (Game|GetPlayerCharacter 0)))
  (Variables|Default|SetCharacterRef _asbp_character))

(fn ConstructionScript)