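; Base pickup item for equipment, carrying an ItemInfo struct that its construction script stamps with its class and self reference.
; Box overlaps notify BP_Character when the item enters or leaves reach.
; Interaction blocks weighted items when the backpack is full, otherwise routes pickup by item type, weapon type and slot state to body, weapon-slot or general pickup.
; SeeItems overlays a lazily created outline-material mesh copy and sends the item's info to the player.
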(event OnComponentBeginOverlap(BoxComp)
  (params (OverlappedComponent :type Primitive%20Component%20Object%20Reference) (OtherActor :type Actor%20Object%20Reference) (OtherComp :type Primitive%20Component%20Object%20Reference) (OtherBodyIndex :type Integer) (bFromSweep :type Boolean) (SweepResult :type Hit%20Result%20Structure%20%28by%20ref%29))
  (bind _characterref (Variables|Default|GetCharacterRef))
  ;[1 1 1] 交互
  (bind _asbp_character (Utilities|Casting|CastToBP_Character OtherActor))
  (Class|BPInteractive|Meet(Message) _asbp_character self (Variables|Rendering|GetItemInfo))
  ;[1 1 1] 人物里的 “和武器等装备重叠”
  (Utilities|IsValid _characterref
    (:Is%20Valid
      (Default|Overlap _characterref true self))))

(event OnComponentEndOverlap(BoxComp)
  (params (OverlappedComponent :type Primitive%20Component%20Object%20Reference) (OtherActor :type Actor%20Object%20Reference) (OtherComp :type Primitive%20Component%20Object%20Reference) (OtherBodyIndex :type Integer))
  (bind _characterref (Variables|Default|GetCharacterRef))
  ;[1 1 1] 交互
  (bind _asbp_character (Utilities|Casting|CastToBP_Character OtherActor))
  (Class|BPInteractive|Leave(Message) _asbp_character self (Variables|Rendering|GetItemInfo))
  ;[1 1 1] 人物里的 “和武器等装备重叠”
  (Utilities|IsValid _characterref
    (:Is%20Valid
      (Default|Overlap _characterref false self))))

(event EventSeeItems
  (params (Transform :type Transform))
  ;[1 1 1] 注释
  (Utilities|IsValid (Variables|Default|GetOutLine)
    (:Is%20Valid
      _)
    (:Is%20Not%20Valid
      ;;[1 1 1] 判断，看见物品后生成放光的边框
      (bind _returnvalue (AddComponent|AddStaticMeshComponent false (Math|Transform|MakeTransform "0, 0, 0" (.rotation Transform) (.scale Transform))))
      (bind _output_get (Variables|Default|SetOutLine _returnvalue))))
  (Components|StaticMesh|SetStaticMesh _output_get (Variables|/Script/Engine.StaticMeshComponent|GetStaticMesh (Variables|Default|GetStaticComp)))
  (Rendering|Material|SetMaterial (Variables|Default|GetOutLine) 0 "/Game/Interface/RPG/Texture/M_Outline_Inst.M_Outline_Inst")
  (Rendering|SetVisibility (Variables|Default|GetOutLine) true false)
  (Transformation|SetWorldTransform (Variables|Default|GetOutLine) (Transformation|GetWorldTransform (Variables|Default|GetStaticComp)) false false)
  (Class|BPInteractive|NearbyItemInfo(Message) (Game|GetPlayerCharacter 0) (Variables|Rendering|GetItemInfo)))

(event EventBeginPlay
  ;[1 1 1] 初始化
  (bind _asbp_character (Utilities|Casting|CastToBP_Character (Game|GetPlayerCharacter 0)))
  (Variables|Default|SetCharacterRef _asbp_character))

(event EventInteraction
  (params (Char :type Object%20Object%20Reference))
  (bind _iteminfo (Variables|Rendering|GetItemInfo))
  (bind _characterref (Variables|Default|GetCharacterRef))
  (bind (_itemtype _weapontype) (Utilities|Struct|BreakBP_ItemInfo _iteminfo))
  ;[1 1 1] 被拾取
  (if (>= (Variables|/Game/Blueprints/BP_Character.BP_Character_C|GetWeight _characterref) (Variables|/Game/Blueprints/BP_Character.BP_Character_C|GetMaxWeight _characterref))
    (if (== (.Weight (Utilities|Struct|BreakBP_ItemInfo (Variables|Rendering|GetItemInfo))) 0)
      ;;[1 1 1] 判断是否是武器和护甲
      (if (Utilities|Enum|Equal(Enum) _itemtype "NewEnumerator1") :!label _label
        (Class|BPInteractive|PickBodyUp(Message) Char _iteminfo)
        (elif (Utilities|Enum|Equal(Enum) _itemtype "NewEnumerator3")
          (Utilities|IsValid (.Image (Utilities|Struct|BreakBP_ItemInfo (Utilities|Array|Get(acopy) (Variables|/Game/Blueprints/BP_Character.BP_Character_C|GetWeaponSlot (Variables|Default|GetCharacterRef)) 4)))
            (:Is%20Valid
              (if (Utilities|Enum|Equal(Enum) _weapontype "NewEnumerator3")
                (Class|BPInteractive|PickUp(Message) Char _iteminfo :!label _label_2)
                (Default|DestroyActor (Variables|Default|GetCharacterRef) self)
                (Development|PrintString "拾取成功??" true true "(R=1.000000,G=0.000000,B=0.000000,A=1.000000)")
                (else
                  (Class|BPInteractive|PickWeaponSlotUp(Message) Char _iteminfo :!label _label_3))))
            (:Is%20Not%20Valid
              (goto _label_3)))
          (else
            (goto _label_2))))
      (else
        (Development|PrintString "背包已经满了")))
    (else
      (goto _label))))

(fn ConstructionScript
  (bind _self self)
  (Utilities|Struct|SetmembersinBP_ItemInfo (Variables|Rendering|GetItemInfo) (Utilities|GetClass _self) _self))