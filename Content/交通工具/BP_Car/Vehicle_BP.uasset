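; Drivable car Blueprint with throttle, steering and handbrake input fed into its VehicleMovement component.
; V toggles between CameraS and first-person CameraY, whose look rotation is clamped each Tick by the misleadingly named ThirdPerson event.
; Tick also sends the larger-magnitude steer angle of wheels 0 and 1 to Vehicle_AnimBlueprint for the steering wheel.
; The construction script makes SkeletalMesh follow the main Mesh's pose via master pose.
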(event Custom|Third%20Person
  (bind _cameray (Variables|Default|GetCameraY))
  (bind _relativerotation (Variables|/Script/Engine.SceneComponent|GetRelativeRotation _cameray))
  (bind (_roll _pitch _yaw) (Math|Rotator|BreakRotator _relativerotation))
  ;[1 1 1] 第三人称视角限制
  (if (Variables|Default|GetIsFirstCamera)
    (Transformation|SetRelativeRotation (Variables|Default|GetCameraY) (Math|Rotator|MakeRotator 0.0 (Math|Float|Clamp(Float) (+ (* (Input|AxisValues|GetLookUp) -1.0) _pitch) -89.0 89.0) (Math|Float|Clamp(Float) (+ _yaw (Input|AxisValues|GetLookRight)) -65.0 65.0)) false false)))

(event Custom|SteeringWheel
  (bind _vehiclemovement (Variables|Default|GetVehicleMovement))
  (bind _wheels (Variables|/Script/PhysXVehicles.WheeledVehicleMovementComponent|GetWheels _vehiclemovement))
  (bind _output (Utilities|Array|Get(acopy) _wheels))
  (bind _output_2 (Utilities|Array|Get(acopy) _wheels 1))
  (bind _returnvalue (Class|VehicleWheel|GetSteerAngle _output))
  (bind _returnvalue_2 (Class|VehicleWheel|GetSteerAngle _output_2))
  ;[1 1 1] 方向盘
  (Variables|/Game/交通工具/BP_Car/Vehicle_AnimBlueprint.Vehicle_AnimBlueprint_C|SetSteeringAngle (Variables|Default|GetAnim%20Ref) (Math|Float|SelectFloat _returnvalue _returnvalue_2 (> (Math|Float|Absolute(Float) _returnvalue) (Math|Float|Absolute(Float) _returnvalue_2)))))

(event EventTick
  (params (DeltaSeconds :type Float%20%28single-precision%29))
  (CallFunction|ThirdPerson)
  (CallFunction|SteeringWheel))

(event EventBeginPlay
  (bind _asvehicle_anim_blueprint (Utilities|Casting|CastToVehicle_AnimBlueprint (Components|SkeletalMesh|GetAnimInstance (Variables|Character|GetMesh))))
  (Variables|Default|SetAnim%20Ref _asvehicle_anim_blueprint))

(event Input|ActionEvents|InputActionHandbrake
  (params (Key :type Key%20Structure))
  (bind _vehiclemovement (Variables|Default|GetVehicleMovement))
  ;[1 1 1] 移动和刹车
  (:Pressed
    (Class|WheeledVehicleMovementComponent|SetHandbrakeInput _vehiclemovement true))
  (:Released
    (Class|WheeledVehicleMovementComponent|SetHandbrakeInput _vehiclemovement false)))

(event Input|AxisEvents|InputAxisLookUp
  (params (AxisValue :type Float%20%28single-precision%29))
  ;[1 1 1] 视角
  (Pawn|Input|AddControllerPitchInput AxisValue))

(event Input|AxisEvents|InputAxisTurn
  (params (AxisValue :type Float%20%28single-precision%29))
  ;[1 1 1] 视角
  (Pawn|Input|AddControllerYawInput AxisValue))

(event Input|AxisEvents|InputAxisMoveForward
  (params (AxisValue :type Float%20%28single-precision%29))
  ;[1 1 1] 移动和刹车
  (Class|WheeledVehicleMovementComponent|SetThrottleInput (Variables|Default|GetVehicleMovement) AxisValue))

(event Input|AxisEvents|InputAxisMoveRight
  (params (AxisValue :type Float%20%28single-precision%29))
  ;[1 1 1] 移动和刹车
  (Class|WheeledVehicleMovementComponent|SetSteeringInput (Variables|Default|GetVehicleMovement) AxisValue))

(event Input|KeyboardEvents|V
  (params (Key :type Key%20Structure))
  ;[1 1 1] 切换视角（第一视角和第二视角）
  (:Pressed
    (Utilities|FlowControl|FlipFlop
      (:A
        (Components|Activation|SetActive (Variables|Default|GetCameraS) false false)
        (Components|Activation|SetActive (Variables|Default|GetCameraY) true false)
        (Variables|Default|SetIsFirstCamera true))
      (:B
        (Components|Activation|SetActive (Variables|Default|GetCameraS) true false)
        (Components|Activation|SetActive (Variables|Default|GetCameraY) false false)
        (Variables|Default|SetIsFirstCamera false)))))

(fn ConstructionScript
  (Class|SkinnedMeshComponent|SetMasterPoseComponent (Variables|Default|GetSkeletalMesh) (Variables|Character|GetMesh) false))