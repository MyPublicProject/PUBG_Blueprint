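; HUD Blueprint that shows an aim-point widget and draws full-screen sniper scope overlays.
; BeginPlay adds the 瞄准点 widget to the viewport, creates dynamic material instances for seven scope styles and caches the player's BP_Character.
; Every DrawHUD picks a scope by the character's BIndex, applies the HUD's ScopeOpacity variable as a material parameter and draws it at screen size.
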(event EventBeginPlay
  (Utilities|FlowControl|Sequence
    (:then_0
      (|创建瞄准点))
    (:then_1
      (|初始化倍镜))
    (:then_2
      (bind _asbp_character (Utilities|Casting|CastToBP_Character (Game|GetPlayerCharacter 0)))
      (Variables|Default|SetCharacter%20Ref _asbp_character))))

(event EventDrawHUD
  (params (SizeX :type Integer) (SizeY :type Integer))
  (|选择倍镜 SizeX SizeY))

(fn ConstructionScript)