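; Character customization ("捏脸", face sculpting) Blueprint that opens the whole-body editing UI when play begins.
; BeginPlay adds the UI_WholeBody widget to the viewport, shows the mouse cursor and switches input to UI-only with focus on that widget.
; Tick prints every BodyData entry to the screen as a per-frame debug readout; nothing in this Blueprint writes or applies that data.
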(event EventBeginPlay
  (bind _returnvalue (Game|GetPlayerController 0))
  (bind _returnvalue_2 (UserInterface|CreateWidget "/Game/Interface/StartUI/UI_WholeBody.UI_WholeBody_C" (Game|GetPlayerController 0)))
  (UserInterface|Viewport|AddtoViewport _returnvalue_2 0)
  (Variables|/Script/Engine.PlayerController|SetbShowMouseCursor _returnvalue true)
  (Input|SetInputModeUIOnly _returnvalue _returnvalue_2 "DoNotLock"))

(event EventTick
  (params (DeltaSeconds :type Float%20%28single-precision%29))
  (for _array_element (Variables|Default|GetBodyData)
    (Development|PrintString (Utilities|String|ToString(Float) _array_element) true true "(R=1.000000,G=0.058804,B=0.138485,A=1.000000)" 0.0)))

(fn ConstructionScript)